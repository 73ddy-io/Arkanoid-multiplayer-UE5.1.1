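; Parent brick for a ball-and-brick game that loses life on each BP_Ball hit until destroyed.
; The construction script randomly rolls a life of 1, 2 or 4, which sets material and score.
; Hits refresh both for the remaining life, with no case for 3, so destruction pays the 1-life score.
; On death it fires CubeDestroy with the score and has a 1-in-8 chance to spawn BP_Bonus.
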(event `self.ReceiveBeginPlay`)

(event `self.ReceiveHit`
  (params (MyComp :type "PrimitiveComponent Object Reference") (Other :type "Actor Object Reference") (OtherComp :type "PrimitiveComponent Object Reference") (bSelfMoved :type Boolean) (HitLocation :type "Vector Structure") (HitNormal :type "Vector Structure") (NormalImpulse :type "Vector Structure") (Hit :type "HitResult Structure (by ref)"))
  (cast `/Game/Blueprints/BP_Ball` Other)
  (`self.Ball Collision`))

(event `Ball Collision`
  (bind _result (`/Engine/EditorBlueprintResources/StandardMacros.DecrementInt` (`self.cubeLife`))
    (:`  `
      (if (<= _result 0)
        (`self.cubeDestroy` (`self.cubeScore`))
        (`self.K2_DestroyActor`)
        (if (== (`KismetMathLibrary.RandomIntegerInRange` 1 8) 4)
          (`|SpawnActorFromClass` "/Game/Blueprints/Bricks/Bonus/BP_Bonus.BP_Bonus_C" (`KismetMathLibrary.MakeTransform` (`self.K2_GetActorLocation`)) "AlwaysSpawn" "OverrideRootScale" null null))
        (else
          (`self.setCubeColor`))))))

(fn `setCubeColor`
  (bind _cube (`self.Cube`))
  (switch `int` (`self.cubeLife`)
    (:`1`
      (set `self.cubeScore` 100)
      (`PrimitiveComponent.SetMaterial` _cube 0 "/Game/Materials/M_ColorBase.M_ColorBase"))
    (:`2`
      (set `self.cubeScore` 200)
      (`PrimitiveComponent.SetMaterial` _cube 0 "/Game/Materials/MI_ColorGreen.MI_ColorGreen"))
    (:`4`
      (set `self.cubeScore` 400)
      (`PrimitiveComponent.SetMaterial` _cube 0 "/Game/Materials/MI_ColorPurple.MI_ColorPurple"))))

(fn `setCubeLife`
  (bind _returnvalue (`KismetMathLibrary.RandomIntegerInRange` 1 100))
  (if (<= _returnvalue 60)
    (set `self.cubeLife` 1)
    (elif (<= _returnvalue 90)
      (set `self.cubeLife` 2)
      (else
        (set `self.cubeLife` 4))))
  (`self.setCubeColor`))

(fn `UserConstructionScript`
  (`self.setCubeLife`))