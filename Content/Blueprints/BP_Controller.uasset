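; BP_Controller is the player controller that drives the player's BP_Caret pawn and its ball throw.
; It creates the WBP_HUD widget and sets game-only input on begin play, and caches the caret on possession.
; The Left_Right axis slides the caret along Y with a swept, frame-rate-independent offset scaled by Speed, and Throw_Ball calls the caret's throw event.
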(event `self.ReceiveBeginPlay`
  (`WidgetBlueprintLibrary.SetInputMode_GameOnly` self)
  (bind _returnvalue (`|CreateWidget` "/Game/UI/WBP_HUD.WBP_HUD_C" self))
  (`UserWidget.AddToViewport` _returnvalue 0)
  (set `self.HUD` _returnvalue))

(event `self.ReceivePossess`
  (params (PossessedPawn :type "Pawn Object Reference"))
  (bind _asbp_caret (cast `/Game/Blueprints/BP_Caret` PossessedPawn))
  (set `self.caret` _asbp_caret))

(event `InputAxis|Left_Right`
  (params (AxisValue :type "Float (single-precision)"))
  (`self.K2_AddActorWorldOffset` (`self.caret`) (`KismetMathLibrary.MakeVector` 0.0 (* AxisValue (`GameplayStatics.GetWorldDeltaSeconds`) (`self.speed`))) true false))

(event `InputAction|Throw_Ball`
  (params (Key :type "Key Structure"))
  (:`Pressed`
    (`/Game/Blueprints/BP_Caret.Event ThrowBall` (`self.caret`))))

(fn `UserConstructionScript`)