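; Grid generator actor that randomly scatters BP_BrickCommon bricks over a grid at BeginPlay and routes their destruction score to BP_Caret.
; Each cell, spaced by Gap from the actor's location, has a small random chance to spawn a brick into CubeArray.
; After each row of the outer loop, it updates CubeArrayCount and binds every brick's CubeDestroy event to AddScore.
; Static-mesh grid construction and cleanup logic is present but disconnected.
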(event `self.ReceiveBeginPlay`
  (bind (_returnvalue_x _returnvalue_y _returnvalue_z) (`KismetMathLibrary.BreakVector` (`self.K2_GetActorLocation`)))
  (`|ExecutionSequence`
    (:`then_0`
      (bind _returnvalue (`GameplayStatics.GetActorOfClass` "/Game/Blueprints/BP_Caret.BP_Caret_C"))
      (set `self.caret` _returnvalue))
    (:`then_1`
      (for _index (range (+ (`self.offsetX`) 1))
        (for _index_2 (range (+ (`self.offsetY`) 1))
          (if (<= (`KismetMathLibrary.RandomIntegerInRange` 1 10) 1)
            (bind _returnvalue_2 (`|SpawnActorFromClass` "/Game/Blueprints/Bricks/BP_BrickCommon.BP_BrickCommon_C" (`KismetMathLibrary.MakeTransform` (`KismetMathLibrary.MakeVector` (+ (`KismetMathLibrary.Conv_IntToDouble` (* _index (`self.gap`))) _returnvalue_x) (+ (`KismetMathLibrary.Conv_IntToDouble` (* _index_2 (`self.gap`))) _returnvalue_y) _returnvalue_z)) "Undefined" "OverrideRootScale" null null))
            (`KismetArrayLibrary.Array_Add` (`self.cubeArray`) _returnvalue_2)))
        (bind _cubearraycount (`self.getCubeArrayCount`))
        (set `self.cubeArrayCount` _cubearraycount)
        (for _array_element (`self.cubeArray`)
          (add `/Game/Blueprints/Bricks/BP_BrickParent.cubeDestroy` _array_element (delegate `Event AddScore`)))))))

(event `Event AddScore`
  (params (cubeScore :type Integer))
  (`/Game/Blueprints/BP_Caret.addScore` (`self.caret`) cubeScore))

(fn `getCubeArrayCount`
  (returns (cubeArrayCount :type Integer))
  (return (`KismetArrayLibrary.Array_Length` (`self.cubeArray`))))

(fn `UserConstructionScript`)